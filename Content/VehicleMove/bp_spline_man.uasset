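; Spline actor that moves a skeletal mesh along a path, likely a walking character judging by its name.
; Timeline T1 maps its track to spline distance, setting the mesh's location and rotation with a -90 yaw offset and applying a configurable play rate.
; The construction script applies the chosen skeletal mesh.
; No event in the graph starts the timeline, so movement depends on autoplay or an external trigger.
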(fn `UserConstructionScript`
  (`SkinnedMeshComponent.SetSkinnedAssetAndUpdate` (`self.A1`) (`self.New mesh`) true))